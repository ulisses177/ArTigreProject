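; Spline-driven pipe prop that builds a continuous pipe along an editable spline.
; The construction script adds one collidable spline mesh per segment between neighboring points, using their local locations and tangents.
; Diameter and CanoTigre (MetalPlastic or Glass) select each segment's mesh, and CanoTigre also selects its material.
; A shared SplineUpDir is applied to every segment to control its orientation.
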(fn `UserConstructionScript`
  (bind _spline (`self.Spline`))
  (bind _canotigre (`self.CanoTigre`))
  ;[1 1 1] Create the Spline Meshes for each node of the spline, and apply the Spline Up Direction
  (for _index (range (+ (- (`SplineComponent.GetNumberOfSplinePoints` _spline) 2) 1))
    (bind _returnvalue (`AddComponent|NODE_AddSplineMeshComponent-0` :`bManualAttachment` true))
    (`StaticMeshComponent.SetStaticMesh` _returnvalue (select `int` (`self.Diameter`) :`0` null :`1` (select `/Game/TigreProps/Enum_CanoTigre` _canotigre :`NewEnumerator0` "/Game/TigreProps/TigreSplinePipeSegment1_2.TigreSplinePipeSegment1_2" :`NewEnumerator1` "/Game/TigreProps/TigreTubeSplineMesh01_2.TigreTubeSplineMesh01_2" :!type "StaticMesh Object Reference") :`2` (select `/Game/TigreProps/Enum_CanoTigre` _canotigre :`NewEnumerator0` "/Game/TigreProps/TigreSplinePipeSegment2_2.TigreSplinePipeSegment2_2" :`NewEnumerator1` "/Game/TigreProps/TigreTubeSplineMesh02_2.TigreTubeSplineMesh02_2" :!type "StaticMesh Object Reference") :`3` (select `/Game/TigreProps/Enum_CanoTigre` _canotigre :`NewEnumerator0` "/Game/TigreProps/TigreSplinePipeSegment3_2.TigreSplinePipeSegment3_2" :`NewEnumerator1` "/Game/TigreProps/TigreTubeSplineMesh03_2.TigreTubeSplineMesh03_2" :!type "StaticMesh Object Reference") :`4` (select `/Game/TigreProps/Enum_CanoTigre` _canotigre :`NewEnumerator0` "/Game/TigreProps/TigreSplinePipeSegment4_2.TigreSplinePipeSegment4_2" :`NewEnumerator1` "/Game/TigreProps/TigreTubeSplineMesh04_2.TigreTubeSplineMesh04_2" :!type "StaticMesh Object Reference")))
    (`PrimitiveComponent.SetMaterial` _returnvalue 0 (select `/Game/TigreProps/Enum_CanoTigre` (`self.CanoTigre`) :!type "MaterialInstanceDynamic Object Reference"))
    (`PrimitiveComponent.SetCollisionEnabled` _returnvalue "QueryAndPhysics")
    (`SceneComponent.K2_AttachToComponent` _returnvalue (`self.SceneRoot`) "None" "KeepRelative" "KeepRelative" "KeepRelative" true)
    (bind (_location _tangent) (`SplineComponent.GetLocationAndTangentAtSplinePoint` _spline _index "Local"))
    (bind (_location_2 _tangent_2) (`SplineComponent.GetLocationAndTangentAtSplinePoint` _spline (+ _index 1) "Local"))
    (`SplineMeshComponent.SetStartAndEnd` _returnvalue _location _tangent _location_2 _tangent_2 true)
    (`SplineMeshComponent.SetSplineUpDir` _returnvalue (`self.SplineUpDir`) true)))